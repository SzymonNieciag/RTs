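; Character Blueprint using gameplay abilities and attributes, with team identity, a health bar and a toggleable decal.
; On BeginPlay it passes its team to BP_MainController, feeds that ID into a dynamic mesh material and acquires GA_Shot.
; Health changes set the widget bar to max health divided by current health, and death detaches the controller pending destroy.
; Tick and the decal events also print debug strings.
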(event `self.ReceiveBeginPlay`
  (bind _mainmesh (`self.MainMesh`))
  (bind _asbp_main_controller (cast `/Game/BP_MainController` (`self.GetController`)))
  (`MainCharacterController.SetGenericTeamId` _asbp_main_controller (`self.team`))
  (bind _returnvalue (`KismetMaterialLibrary.CreateDynamicMaterialInstance` "/Game/globe_puzzle_A.globe_puzzle_A"))
  (`PrimitiveComponent.SetMaterial` _mainmesh 0 _returnvalue)
  (bind _returnvalue_teamid (break `GenericTeamId` (`MainCharacterController.GetGenericTeamId` _asbp_main_controller)))
  (`MeshComponent.SetVectorParameterValueOnMaterials` _mainmesh "Param" (`KismetMathLibrary.MakeVector` (`KismetMathLibrary.Conv_IntToDouble` (`KismetMathLibrary.Conv_ByteToInt` _returnvalue_teamid))))
  (`self.AquireAbility` "/Game/Blueprints/Ability/GA_Shot.GA_Shot_C"))

(event `self.ReceiveTick`
  (params (DeltaSeconds :type "Float (single-precision)"))
  (bind _health_basevalue (break `GameplayAttributeData` (`AttributeSetBase.Health` (`self.AttributeSetBase`))))
  (`KismetSystemLibrary.Delay` 0.2)
  (`KismetSystemLibrary.PrintString` (`KismetStringLibrary.Conv_DoubleToString` _health_basevalue)))

(event `self.EnableDecalEffect`
  (`KismetSystemLibrary.PrintString` "visible")
  (`SceneComponent.SetVisibility` (`self.Decal`) true false))

(event `self.DisableDecalEffect`
  (`KismetSystemLibrary.PrintString` "Hello")
  (`SceneComponent.SetVisibility` (`self.Decal`) false false))

(event `self.OnHealtChanged`
  (params (DeltaValue :type "Float (single-precision)") (EventTags :type "GameplayTagContainer Structure (by ref)"))
  (bind _aswbp_health_bar (cast `/Game/Blueprints/Widgets/WBP_HealthBar` (`WidgetComponent.GetUserWidgetObject` (`self.HealthBar`))))
  (`ProgressBar.SetPercent` (`/Game/Blueprints/Widgets/WBP_HealthBar.ProgressBar_120` _aswbp_health_bar) (/ (`self.GetMaxHealth`) (`self.GetHealth`))))

(event `self.OnDeath`
  (`self.DetachFromControllerPendingDestroy`))

(fn `UserConstructionScript`)