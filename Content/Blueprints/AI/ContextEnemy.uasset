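; ContextEnemy is an EQS query context that supplies enemy actors to environment queries.
; ProvideActorsSet returns every TestPawn in the level, whichever querier runs the query.
; ProvideSingleActor has an empty body, with disconnected logic that would read the querier's "Enemy" Blackboard value.
; A disconnected lookup of all BP_MainCharacter actors also remains in the set graph.
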(fn `ProvideActorsSet`
  (params (QuerierObject :type "Object Object Reference") (QuerierActor :type "Actor Object Reference"))
  (returns (ResultingActorsSet :type "Array of Actor Object Reference"))
  (bind _outactors (`GameplayStatics.GetAllActorsOfClass` "/Game/Blueprints/AI/testPawn.testPawn_C"))
  (return _outactors))

(fn `ProvideSingleActor`
  (params (QuerierObject :type "Object Object Reference") (QuerierActor :type "Actor Object Reference"))
  (returns (ResultingActor :type "Actor Object Reference")))