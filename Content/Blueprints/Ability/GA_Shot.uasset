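; GA_Shot is a Gameplay Ability that resolves a shot's damage with a percentage hit roll.
; On activation it commits, then waits for a Shot.Damage gameplay event carrying the instigator and target.
; The instigating MainCharacter calculates hit chance against the target, and a successful random roll applies GE_ShotDamage to it.
; The ability ends after a hit or miss, but stays active if the MainCharacter cast fails.
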(event `self.K2_ActivateAbility`
  (`self.K2_CommitAbility`)
  (bind (_asynctaskproxy _payload) (`AbilityTask_WaitGameplayEvent.WaitGameplayEvent` (struct :`TagName` "shot.Damage") null)
    (:`EventReceived`
      (bind _asmain_character (cast `MainCharacter` (`.Instigator` (break `GameplayEventData` _payload))))
      (bind _returnvalue (`MainCharacter.CalculateChanceToHitTarget` _asmain_character (`.Target` (break `GameplayEventData` _payload))))
      (if (>= _returnvalue (`KismetMathLibrary.RandomFloatInRange` 0.0 100.0))
        (`self.BP_ApplyGameplayEffectToTarget` (`AbilitySystemBlueprintLibrary.AbilityTargetDataFromActor` (`.Target` (break `GameplayEventData` _payload))) "/Game/Blueprints/Ability/GE_ShotDamage.GE_ShotDamage_C")
        (`self.K2_EndAbility`)
        (else
          (`self.K2_EndAbility`))))))