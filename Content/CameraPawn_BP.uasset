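; Camera pawn that handles mouse-wheel zoom on a spring arm, tilting the view as the arm length changes.
; BeginPlay captures the boom's initial length as the maximum zoom and its initial pitch as one angle limit.
; Wheel input adjusts clamped target values for length and pitch independently.
; Tick eases the boom toward both targets with a fixed-alpha Lerp, so smoothing depends on frame rate.
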(event `self.ReceiveBeginPlay`
  (bind (_relativerotation_roll _relativerotation_pitch) (`KismetMathLibrary.BreakRotator` (`SceneComponent.RelativeRotation` (`self.CameraBoom`))))
  (bind _targetarmlength (`SpringArmComponent.TargetArmLength` (`self.CameraBoom`)))
  (set `self.StartRakeAngleArm` _relativerotation_pitch)
  (set `self.CurrentRakeAngleArm` _relativerotation_pitch)
  (set `self.MaxHeightArm` _targetarmlength)
  (set `self.CurrentHeightArm` _targetarmlength))

(event `InputAxisKey|MouseWheelAxis`
  (params (AxisValue :type "Float (single-precision)"))
  (`|ExecutionSequence`
    (:`then_0`
      (set `self.CurrentHeightArm` (`KismetMathLibrary.FClamp` (+ (* AxisValue (`self.LerpSpeedZoom`)) (`self.CurrentHeightArm`)) (`self.MinHeightArm`) (`self.MaxHeightArm`))))
    (:`then_1`
      (set `self.CurrentRakeAngleArm` (`KismetMathLibrary.FClamp` (+ (* AxisValue (`self.LerpSpeedAngle`)) (`self.CurrentRakeAngleArm`)) (`self.StartRakeAngleArm`) (`self.FinishRakeAngleArm`))))))

(event `self.ReceiveTick`
  (params (DeltaSeconds :type "Float (single-precision)"))
  (bind _cameraboom (`self.CameraBoom`))
  (bind _cameraboom_2 (`self.CameraBoom`))
  (bind (_relativerotation_roll _relativerotation_pitch) (`KismetMathLibrary.BreakRotator` (`SceneComponent.RelativeRotation` _cameraboom)))
  (set `SpringArmComponent.TargetArmLength` (`KismetMathLibrary.Lerp` (`SpringArmComponent.TargetArmLength` _cameraboom_2) (`self.CurrentHeightArm`) 0.02) _cameraboom_2)
  (`SceneComponent.K2_SetRelativeRotation` _cameraboom (`KismetMathLibrary.MakeRotator` 0.0 (`KismetMathLibrary.Lerp` _relativerotation_pitch (`self.CurrentRakeAngleArm`) 0.02)) false false))

(fn `UserConstructionScript`)