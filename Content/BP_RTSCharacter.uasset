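; RTS unit character with team identity, a weapon, a shot ability and selection feedback.
; On BeginPlay it passes its team ID to its BP_MainController, sets the team body material, acquires GA_Shot and spawns its weapon.
; Events toggle the selection decal, flash a retriggerable preview decal, update the health bar and show floating damage numbers.
; Death detaches the controller, plays an animation and removes the selection decal and health bar.
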(event `self.ReceiveBeginPlay`
  (bind _mesh (`self.Mesh`))
  (bind _asbp_main_controller (cast `/Game/BP_MainController` (`self.GetController`)))
  (`MainCharacterController.SetGenericTeamId` _asbp_main_controller (make `GenericTeamId` (`self.TeamID`)))
  (`|ExecutionSequence`
    (:`then_0`
      (switch `ETeamType` (`self.TeamID`)
        (:`Red`
          (`PrimitiveComponent.SetMaterial` _mesh 0 "/Game/Mannequin/Character/Materials/Body_1.Body_1"))
        (:`Blue`
          (`PrimitiveComponent.SetMaterial` _mesh 0 "/Game/Mannequin/Character/Materials/Body_2.Body_2"))))
    (:`then_1`
      (`self.AquireAbility` "/Game/Blueprints/Ability/GA_Shot.GA_Shot_C")
      (bind _returnvalue (`|SpawnActorFromClass` (`self.WeaponClass`) (`KismetMathLibrary.MakeTransform` (0.0 0.0 0.0)) "Undefined" "OverrideRootScale" null null))
      (bind _output_get (set `self.Weapon` _returnvalue))
      (`KismetSystemLibrary.PrintString` (`KismetStringLibrary.Conv_DoubleToString` (`Weapon.GetWeaponDamage` _output_get))))))

(event `self.ReTriggerPreviewDecal`
  (bind _decal1 (`self.Decal1`))
  (`SceneComponent.SetVisibility` _decal1 true false)
  (`KismetSystemLibrary.RetriggerableDelay` 0.2)
  (`SceneComponent.SetVisibility` _decal1 false false))

(event `self.EnableSelectedDecal`
  (bind _decal (`self.Decal`))
  (`/Engine/EditorBlueprintResources/StandardMacros.IsValid` _decal
    (:`Is Valid`
      (`SceneComponent.SetVisibility` _decal true false))))

(event `self.DisableSelectedDecal`
  (bind _decal (`self.Decal`))
  (`/Engine/EditorBlueprintResources/StandardMacros.IsValid` _decal
    (:`Is Valid`
      (`SceneComponent.SetVisibility` _decal false false))))

(event `self.OnHealtChanged`
  (params (DeltaValue :type "Float (single-precision)") (EventTags :type "GameplayTagContainer Structure (by ref)"))
  (bind _health_bar (`self.Health Bar`))
  (`/Engine/EditorBlueprintResources/StandardMacros.IsValid` _health_bar
    (:`Is Valid`
      (bind _aswbp_health_bar (cast `/Game/Blueprints/Widgets/WBP_HealthBar` (`WidgetComponent.GetUserWidgetObject` _health_bar)))
      (`ProgressBar.SetPercent` (`/Game/Blueprints/Widgets/WBP_HealthBar.ProgressBar_120` _aswbp_health_bar) (/ (`self.GetHealth`) (`self.GetMaxHealth`))))))

(event `self.OnDeath`
  (`self.DetachFromControllerPendingDestroy`)
  (`SkeletalMeshComponent.PlayAnimation` (`self.Mesh`) "/Game/Deaths/Animation/Deaths_Gut_Shot.Deaths_Gut_Shot" false)
  (`ActorComponent.K2_DestroyComponent` (`self.Decal`))
  (`ActorComponent.K2_DestroyComponent` (`self.Health Bar`)))

(event `self.OnDamaged`
  (params (DamageAmount :type "Float (single-precision)") (HitInfo :type "HitResult Structure (by ref)") (DamageTags :type "GameplayTagContainer Structure (by ref)") (InstigatorCharacter :type "RTSCharacter Object Reference") (DamageCauser :type "Actor Object Reference"))
  (bind _returnvalue (`GameplayStatics.GetPlayerController` 0))
  (bind _returnvalue_2 (`|CreateWidget` "/Game/Blueprints/Widgets/WBP_FloatingDamage.WBP_FloatingDamage_C" _returnvalue (`PlayerController.ProjectWorldLocationToScreen` _returnvalue (`self.K2_GetActorLocation`) false) DamageAmount))
  (`UserWidget.AddToViewport` _returnvalue_2 0))

(fn `UserConstructionScript`)